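; Ghost actor for the Pseudoregalia multiplayer mod, showing a tinted Sybil mesh with a floating name label.
; On BeginPlay, it writes Color and Intensity into the mesh's DieColor and DieAmount material parameters and sets the label text from Name.
; Each Tick, it turns the label toward the player camera and scales it with camera distance, never below unit size.
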(event EventTick
  (params (DeltaSeconds :type Float%20%28single-precision%29))
  (bind _returnvalue (Game|GetPlayerCameraManager 0))
  (bind _textrender (Variables|Default|GetTextRender))
  (bind _returnvalue_2 (Transformation|GetWorldLocation _textrender))
  (bind _transformcomponent (Variables|/Script/Engine.PlayerCameraManager|GetTransformComponent _returnvalue))
  (bind _returnvalue_3 (Transformation|GetWorldLocation _transformcomponent))
  (bind _returnvalue_4 (Math|Vector|Distance(Vector) _returnvalue_2 _returnvalue_3))
  (bind _returnvalue_5 (* _returnvalue_4 0.003))
  (bind _returnvalue_6 (Math|Float|Max(Float) _returnvalue_5 1.0))
  (Transformation|SetWorldRotation _textrender (Math|Rotator|FindLookatRotation _returnvalue_2 _returnvalue_3) false false)
  (Transformation|SetWorldScale3D _textrender (Math|Vector|MakeVector _returnvalue_6 _returnvalue_6 _returnvalue_6)))

(event EventBeginPlay
  (bind _sybilmesh (Variables|Default|GetsybilMesh))
  (Rendering|Material|SetVectorParameterValueonMaterials _sybilmesh "DieColor" (Math|Conversions|ToVector(LinearColor) (Variables|Default|GetColor)))
  (Rendering|Material|SetScalarParameterValueonMaterials _sybilmesh "DieAmount" (Variables|Default|GetIntensity))
  (Rendering|Components|TextRender|SetText (Variables|Default|GetTextRender) (Utilities|Text|ToText(String) (Variables|Default|GetName))))

(fn ConstructionScript)